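; BP_ColorsPlatform is a platform that cycles its color like a traffic light and changes the speed of the player standing on it.
; A looping BeginPlay sequence drives a dynamic material: a green hold, a timeline-driven gray-to-yellow blink, then a red hold.
; The box overlap tracks the third-person character; Tick varies its Speed with the blink and zeroes it on red.
; Leaving the box restores a fixed speed.
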(event OnComponentBeginOverlap(Box)
  (params (OverlappedComponent :type Primitive%20Component%20Object%20Reference) (OtherActor :type Actor%20Object%20Reference) (OtherComp :type Primitive%20Component%20Object%20Reference) (OtherBodyIndex :type Integer) (bFromSweep :type Boolean) (SweepResult :type Hit%20Result%20Structure%20%28by%20ref%29))
  (bind _asbp_third_person_character (Utilities|Casting|CastToBP_ThirdPersonCharacter OtherActor))
  (Variables|Default|SetPlayerRef _asbp_third_person_character))

(event OnComponentEndOverlap(Box)
  (params (OverlappedComponent :type Primitive%20Component%20Object%20Reference) (OtherActor :type Actor%20Object%20Reference) (OtherComp :type Primitive%20Component%20Object%20Reference) (OtherBodyIndex :type Integer))
  (Utilities|Casting|CastToBP_ThirdPersonCharacter OtherActor)
  (Variables|/Game/Blueprints/ThirdP_BP/BP_ThirdPersonCharacter.BP_ThirdPersonCharacter_C|SetSpeed (Variables|Default|GetPlayerRef) 7e+02)
  (Variables|Default|SetPlayerRef 0))

(event EventBeginPlay
  (bind _returnvalue (Rendering|Material|CreateDynamicMaterialInstance "/Game/Materials/M_Color_Platform.M_Color_Platform" "None" "None" :!class /Script/Engine.KismetMaterialLibrary))
  (bind _output_get (Variables|Default|SetMaterialColor _returnvalue))
  (Rendering|Material|SetMaterial (Variables|Default|GetCube) 0 _output_get)
  (Rendering|Material|SetVectorParameterValue (Variables|Default|GetMaterialColor) "Param" "(R=0.246236,G=1.000000,B=0.019858,A=1.000000)" :!class /Script/Engine.MaterialInstanceDynamic :!label _label)
  (Utilities|FlowControl|Delay 1e+01)
  (bind _newtrack_0 (Timeline|Blinking PlayFromStart)
    (:Update
      ;[0.15 0.15 0.15 0.5] Speed variation linked to blink
      (bind _output_get_2 (Variables|Default|SetColorTrack _newtrack_0))
      (Rendering|Material|SetVectorParameterValue (Variables|Default|GetMaterialColor) "Param" (Math|Color|Lerp(LinearColor) (Variables|Default|GetGray) (Variables|Default|GetYellow) _output_get_2) :!class /Script/Engine.MaterialInstanceDynamic)
      (Variables|Default|SetIsPlaying true))
    (:Finished
      (Development|PrintString "END" true true "(R=0.000000,G=0.660000,B=1.000000,A=1.000000)" 1.0)
      (Variables|Default|SetIsPlaying false)
      (Rendering|Material|SetVectorParameterValue (Variables|Default|GetMaterialColor) "Param" (Variables|Default|GetRed) :!class /Script/Engine.MaterialInstanceDynamic)
      (Variables|Default|SetIsRed true)
      (Utilities|FlowControl|Delay 1e+01)
      (Variables|Default|SetIsRed false)
      (goto _label))))

(event EventTick
  (params (DeltaSeconds :type Float%20%28single-precision%29))
  (bind _playerref (Variables|Default|GetPlayerRef))
  ;[0.15 0.15 0.15 0.5] Changement de speed selon color
  (Utilities|IsValid _playerref
    (:Is%20Valid
      (if (Variables|Default|GetIsRed)
        (Variables|/Game/Blueprints/ThirdP_BP/BP_ThirdPersonCharacter.BP_ThirdPersonCharacter_C|SetSpeed _playerref 0.0)
        (elif (Variables|Default|GetIsPlaying)
          (Variables|/Game/Blueprints/ThirdP_BP/BP_ThirdPersonCharacter.BP_ThirdPersonCharacter_C|SetSpeed _playerref (Math|Float|Lerp 5e+02 3.5e+02 (Variables|Default|GetColorTrack))))))))

(fn ConstructionScript
  (|CallParentFunction))