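; BP_Target is an NPC target whose mesh travels along a spline and splits when a dashing player hits it.
; Tick advances the spline distance by Speed, moves the mesh there and prints a debug string.
; Box overlap with a dashing BP_ThirdPersonCharacter clears and hides the mesh and shows the CoteD and CoteG halves, logic flagged as not working.
; BeginPlay requests a random navigable location but leaves it unused.
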(event OnComponentBeginOverlap(Box)
  (params (OverlappedComponent :type Primitive%20Component%20Object%20Reference) (OtherActor :type Actor%20Object%20Reference) (OtherComp :type Primitive%20Component%20Object%20Reference) (OtherBodyIndex :type Integer) (bFromSweep :type Boolean) (SweepResult :type Hit%20Result%20Structure%20%28by%20ref%29))
  (bind _mesh (Variables|Character|GetMesh))
  ;[0.15 0.15 0.15 0.5] Marche pas (ordre à revoir d'après Louis)
  (bind _asbp_third_person_character (Utilities|Casting|CastToBP_ThirdPersonCharacter OtherActor))
  (if (Variables|/Game/Blueprints/ThirdP_BP/BP_ThirdPersonCharacter.BP_ThirdPersonCharacter_C|GetIsDashing _asbp_third_person_character)
    (Components|SkeletalMesh|SetSkeletalMeshAsset _mesh 0)
    (Rendering|SetVisibility _mesh false false)
    (Rendering|SetVisibility (Variables|Default|GetCoteD) true false)
    (Rendering|SetVisibility (Variables|Default|GetCoteG) true false)))

(event EventBeginPlay
  (Class|NavigationSystemV1|GetRandomLocationinNavigableRadius "0, 0, 0" 0.0 0 0))

(event EventTick
  (params (DeltaSeconds :type Float%20%28single-precision%29))
  ;[0.15 0.15 0.15 0.5] Marche pas (ordre à revoir d'après Louis)
  (Variables|Default|SetDistance%20along%20spline (+ (* DeltaSeconds (Variables|Default|GetSpeed)) (Variables|Default|GetDistance%20along%20spline)))
  (Development|PrintString "WO")
  (Transformation|SetRelativeTransform (Variables|Character|GetMesh) (Math|Transform|MakeTransform (.location (Spline|GetTransformatDistanceAlongSpline (Variables|Default|GetSpline) (Variables|Default|GetDistance%20along%20spline) "Local" false)) (.rotation (Spline|GetTransformatDistanceAlongSpline (Variables|Default|GetSpline) (Variables|Default|GetDistance%20along%20spline) "Local" false)) (Variables|/Script/Engine.SceneComponent|GetRelativeScale3D (Variables|Character|GetMesh))) false false))

(fn ConstructionScript)