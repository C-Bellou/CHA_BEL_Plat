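; BP_Monster is an NPC enemy that chases pawns it sees and hurts the player on contact.
; A PawnSensing component feeds each seen pawn to AI MoveTo as the target to follow.
; A Box overlap applies fixed damage to BP_ThirdPersonCharacter only, with debug prints around the hit.
; An empty Timeline and a second character cast reading HP are unconnected leftovers that never run.
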(event OnSeePawn(PawnSensing)
  (params (Pawn :type Pawn%20Object%20Reference))
  (Utilities|FlowControl|Sequence
    (:then_0
      (AI|AIMoveTo self "0, 0, 0" Pawn 5.0 false))))

(event OnComponentBeginOverlap(Box)
  (params (OverlappedComponent :type Primitive%20Component%20Object%20Reference) (OtherActor :type Actor%20Object%20Reference) (OtherComp :type Primitive%20Component%20Object%20Reference) (OtherBodyIndex :type Integer) (bFromSweep :type Boolean) (SweepResult :type Hit%20Result%20Structure%20%28by%20ref%29))
  (bind _asbp_third_person_character (Utilities|Casting|CastToBP_ThirdPersonCharacter OtherActor))
  (Development|PrintString "Over")
  (Game|Damage|ApplyDamage _asbp_third_person_character 3e+01 0 0)
  (Development|PrintString "OUCH"))

(event EventBeginPlay)

(event Collision|EventActorBeginOverlap
  (params (OtherActor :type Actor%20Object%20Reference)))

(event EventTick
  (params (DeltaSeconds :type Float%20%28single-precision%29)))

(fn ConstructionScript)